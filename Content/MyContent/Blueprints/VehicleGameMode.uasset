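; VehicleGameMode is a game mode Blueprint that respawns the player's Sedan after it is destroyed.
; On BeginPlay it casts player pawn 0 to Sedan and binds a handler to its OnDestroyed event.
; The handler waits briefly, spawns a new Sedan at the SpawnTransform variable, possesses it with player controller 0, then calls Respawn to rebind, so the cycle repeats.
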(event `Respawn`
  (bind _assedan (cast `/Game/MyContent/Sedan/Sedan` (`GameplayStatics.GetPlayerPawn` 0) :!label _label))
  (add `self.OnDestroyed` _assedan (delegate `onDestroy`)))

(event `self.ReceiveBeginPlay`
  (goto _label))

(event `onDestroy` :!signature `self.OnDestroyed`
  (params (DestroyedActor :type "Actor Object Reference"))
  (`KismetSystemLibrary.Delay` 1.0)
  (bind _returnvalue (`|SpawnActorFromClass` "/Game/MyContent/Sedan/Sedan.Sedan_C" (`self.Spawn Transform`) "AdjustIfPossibleButAlwaysSpawn" "OverrideRootScale" null null))
  (`Controller.Possess` (`GameplayStatics.GetPlayerController` 0) _returnvalue)
  (`self.Respawn`))

(fn `UserConstructionScript`)