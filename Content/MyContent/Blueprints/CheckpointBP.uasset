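; CheckpointBP is a checkpoint that a Sedan clears by driving through it in the correct direction.
; On trigger overlap, it takes the dot product of the car's velocity and the Arrow component's forward vector, accepting only positive results.
; A valid pass calls CheckPointCleared with the checkpoint number, hides the trigger, particles, cube and arrow, and disables overlap events so it cannot fire again.
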(event `self.trigger.OnComponentBeginOverlap`
  (params (OverlappedComponent :type "PrimitiveComponent Object Reference") (OtherActor :type "Actor Object Reference") (OtherComp :type "PrimitiveComponent Object Reference") (OtherBodyIndex :type Integer) (bFromSweep :type Boolean) (SweepResult :type "HitResult Structure (by ref)"))
  (bind _trigger (`self.trigger`))
  ;[1 1 1] Checkpoint system - Clears when overlapped, can only clear checkpoints the right way
  (bind _assedan (cast `/Game/MyContent/Sedan/Sedan` OtherActor))
  (if (> (`KismetMathLibrary.Dot_VectorVector` (`self.GetVelocity` _assedan) (`KismetMathLibrary.Conv_RotatorToVector` (`SceneComponent.K2_GetComponentRotation` (`self.Arrow`)))) 0.0)
    (`self.CheckPointCleared` (`self.CheckPointNumber`))
    (`SceneComponent.SetHiddenInGame` _trigger true false)
    (`SceneComponent.SetHiddenInGame` (`self.ParticleSystem`) true false)
    (`SceneComponent.SetHiddenInGame` (`self.Cube`) true false)
    (`SceneComponent.SetHiddenInGame` (`self.Arrow`) true false)
    (set `PrimitiveComponent.bGenerateOverlapEvents` false _trigger)))

(fn `UserConstructionScript`)